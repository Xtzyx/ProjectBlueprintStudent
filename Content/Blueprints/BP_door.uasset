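; BP_door is an interactable double door that swings open and shut with sound.
; BeginPlay stores the starting rotations of two scene pivots, Scene and Scene1.
; When Interagir fires and Close is false, a FlipFlop alternates between playing and reversing the Chronologie timeline, each with its own 2D sound.
; The timeline's Open track, scaled by Angle, yaws the pivots in opposite directions from their stored rotations.
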(event EventBeginPlay
  (Variables|Default|SetPD (Variables|/Script/Engine.SceneComponent|GetRelativeRotation (Variables|Default|GetScene)))
  (Variables|Default|SetPG (Variables|/Script/Engine.SceneComponent|GetRelativeRotation (Variables|Default|GetScene1))))

(event Collision|EventActorBeginOverlap
  (params (OtherActor :type Actor%20Object%20Reference)))

(event EventTick
  (params (DeltaSeconds :type Float%20%28single-precision%29)))

(event EventInteragir
  (bind _pd (Variables|Default|GetPD))
  (bind _pg (Variables|Default|GetPG))
  (if (not (Variables|Default|GetClose?))
    (Utilities|FlowControl|FlipFlop
      (:A
        (Audio|PlaySound2D "/Game/Audio/dooropened-103851.dooropened-103851" 1.0 1.0 0.0 0 0)
        (bind _open (Timeline|Chronologie Play)
          (:Update
            (Transformation|SetRelativeRotation (Variables|Default|GetScene) (Math|Rotator|MakeRotator (.roll _pd) (.pitch _pd) (+ (.yaw _pd) (* _open (Variables|Default|GetAngle)))) false false)
            (Transformation|SetRelativeRotation (Variables|Default|GetScene1) (Math|Rotator|MakeRotator (.roll _pg) (.pitch _pg) (+ (.yaw _pg) (* (* _open (Variables|Default|GetAngle)) -1.0))) false false))))
      (:B
        (Audio|PlaySound2D "/Game/Audio/door-close-79921.door-close-79921" 1.0 1.0 0.0 0 0)
        (Timeline|Chronologie Reverse)))))

(fn ConstructionScript)